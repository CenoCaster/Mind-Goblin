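; NPC man character that patrols a list of destinations and reacts comically to being hit.
; On BeginPlay, WalkCyle waits by state, then loops AIMoveTo through Destinations if Walk is set, retrying after failures.
; A capsule hit, gated by DoOnce, launches the mesh with physics impulses and a scream, then plays get-up and yelling montages.
; It resumes walking, then destroys itself with a pop sound; the ScareBox hit event is empty.
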(event `self.ScareBox.OnComponentHit`
  (params (HitComponent :type "PrimitiveComponent Object Reference") (OtherActor :type "Actor Object Reference") (OtherComp :type "PrimitiveComponent Object Reference") (NormalImpulse :type "Vector Structure") (Hit :type "HitResult Structure (by ref)")))

(event `self.CapsuleComponent.OnComponentHit`
  (params (HitComponent :type "PrimitiveComponent Object Reference") (OtherActor :type "Actor Object Reference") (OtherComp :type "PrimitiveComponent Object Reference") (NormalImpulse :type "Vector Structure") (Hit :type "HitResult Structure (by ref)"))
  (bind _mesh (`self.Mesh`))
  (bind _mesh_2 (`self.Mesh`))
  (bind (_relativelocation_x _relativelocation_y) (`KismetMathLibrary.BreakVector` (`SceneComponent.RelativeLocation` _mesh)))
  (`KismetSystemLibrary.PrintString` "hit")
  (`/Engine/EditorBlueprintResources/StandardMacros.DoOnce` false :!label _label
    (:`Completed`
      (`PrimitiveComponent.SetSimulatePhysics` (`self.Mesh`) true)
      (`PrimitiveComponent.AddImpulse` _mesh_2 (0.0 0.0 1000.0) "None" false)
      (`PrimitiveComponent.AddAngularImpulseInDegrees` _mesh_2 (0.0 1000.0 1000.0) "None" false)
      (`GameplayStatics.PlaySound2D` "/Game/AI/Voices_SFX/Man_Scream_03.Man_Scream_03" 1.0 1.0 0.0 null null)
      (`KismetSystemLibrary.Delay` 5.0)
      (`PrimitiveComponent.SetSimulatePhysics` (`self.Mesh`) false)
      (`SceneComponent.K2_SetWorldRotation` _mesh (`KismetMathLibrary.MakeRotator` 0.0) false false)
      (`SceneComponent.K2_SetRelativeLocation` _mesh (`KismetMathLibrary.MakeVector` _relativelocation_x _relativelocation_y 10.0) false false)
      (`self.PlayAnimMontage` "/Game/AI/ManAnimations/getup_Anim_Montage.getup_Anim_Montage")
      (`KismetSystemLibrary.Delay` 0.2)
      (`self.PlayAnimMontage` "/Game/AI/ManAnimations/yelling_Man.yelling_Man")
      (set `self.State` "NewEnumerator0")
      (`KismetSystemLibrary.Delay` 0.2)
      (`self.Walk Cyle`)
      (set `self.State` "NewEnumerator0")
      (`KismetSystemLibrary.Delay` 5.0)
      (`self.K2_DestroyActor`)
      (`GameplayStatics.PlaySound2D` "/Game/AI/Voices_SFX/Minecraft_-_Item_Pop__Sound_Effect__Cue.Minecraft_-_Item_Pop__Sound_Effect__Cue" 1.0 1.0 0.0 null null)
      (goto _label :!via `Reset`))))

(event `Walk Cyle`
  (bind _returnvalue (+ (`self.Target`) 1))
  ;[1 1 1] Checks if we are walking
  (if (not (`|EnumEquality` (`self.State`) "NewEnumerator1"))
    (set `self.State` "NewEnumerator0")
    (`KismetSystemLibrary.Delay` (`self.NPC Waiting Time`)))
  (if (`self.Walk`)
    ;[1 1 1] Created Loop. Will go to all destinations until he the last. Then it will restart
    (`|AIMoveTo` self (0.0 0.0 0.0) (`|GetArrayItem` (`self.Destinations`) (`self.Target`)) :!label _label_2
      (:`OnSuccess`
        (`KismetSystemLibrary.PrintString` "hey this is the thing please repsopmdHello")
        (if (== _returnvalue (`KismetArrayLibrary.Array_Length` (`self.Destinations`)))
          (set `self.Target` 0)
          (goto _label_2)
          (else
            (set `self.Target` _returnvalue)
            (goto _label_2))))
      (:`OnFail`
        (`KismetSystemLibrary.PrintString` "Cry")
        (`KismetSystemLibrary.Delay` 10.0)
        (goto _label_2)))
    (else
      (set `self.State` "NewEnumerator2")
      (`KismetSystemLibrary.Delay` (`KismetMathLibrary.RandomFloatInRange` 2.0 5.0)))))

(event `self.ReceiveBeginPlay`
  (`self.Walk Cyle`))

(fn `UserConstructionScript`)