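; Ship projectile actor built to travel toward a Target along a randomized curved path.
; After a short launch delay, it picks a point along the line to Target, offsets it by random radius and angle, then activates Niagara.
; Gated Tick slides that curve point toward Target while moving the actor with swept constant-speed interpolation.
; A hit or arrival destroys collision and mesh, then the actor after a delay.
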(event `self.Collison.OnComponentHit`
  (params (HitComponent :type "PrimitiveComponent Object Reference") (OtherActor :type "Actor Object Reference") (OtherComp :type "PrimitiveComponent Object Reference") (NormalImpulse :type "Vector Structure") (Hit :type "HitResult Structure (by ref)"))
  (`ActorComponent.K2_DestroyComponent` (`self.Collison`) :!label _label)
  (`ActorComponent.K2_DestroyComponent` (`self.Mesh`))
  (`KismetSystemLibrary.Delay` 1.0)
  (`self.K2_DestroyActor`))

(event `self.ReceiveTick`
  (params (DeltaSeconds :type "Float (single-precision)"))
  (`/Engine/EditorBlueprintResources/StandardMacros.Gate` true :!label _label_2
    (:`Exit`
      (if (!= (`self.K2_GetActorLocation`) (`self.Target`))
        (set `self.EndCurve` (`KismetMathLibrary.VInterpTo_Constant` (`self.EndCurve`) (`self.Target`) (`GameplayStatics.GetWorldDeltaSeconds`) (`self.Speed`)))
        (`self.K2_SetActorLocation` (`KismetMathLibrary.VInterpTo_Constant` (`self.K2_GetActorLocation`) (0.0 0.0 0.0) (`GameplayStatics.GetWorldDeltaSeconds`) (`self.Speed`)) true)
        (else
          (goto _label))))))

(event `self.ReceiveBeginPlay`
  (`KismetSystemLibrary.Delay` 0.2)
  (`self.MidPoint`)
  (`self.Curve`)
  (`ActorComponent.Activate` (`self.Niagara`) false)
  (goto _label_2 :!via `Open`))

(fn `Curve`
  (bind (_x _y) (`KismetMathLibrary.BreakRotIntoAxes` (`KismetMathLibrary.FindLookAtRotation` (`self.Mid`) (`self.Target`))))
  (set `self.EndCurve` (+ (`self.Mid`) (`KismetMathLibrary.RotateAngleAxis` (* _y (`KismetMathLibrary.RandomFloatInRange` (`self.MinCurveRadius`) (`self.MaxCurveRadius`))) (`KismetMathLibrary.RandomFloatInRange` (`self.MinAngle`) (`self.MaxAngle`)) _x))))

(fn `MidPoint`
  (set `self.Mid` (+ (* (- (`self.Target`) (`self.K2_GetActorLocation`)) (`KismetMathLibrary.RandomFloatInRange` (`self.MinCurveDist`) (`self.MaxCurveDist`))) (`self.K2_GetActorLocation`))))

(fn `UserConstructionScript`)